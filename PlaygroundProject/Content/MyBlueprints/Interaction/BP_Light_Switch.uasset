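; BP_Light_Switch is an interactable switch that toggles the visibility of the light components on an array of target lights when interacted with.
; A ray hit highlights its Cube through custom depth and stencil.
; Each hit also sets a short one-shot timer to the ray-miss event, so the highlight clears shortly after hits stop arriving.
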(event `/Game/MyBlueprints/Interaction/Int_Interaction_Highlight.OnRayHit`
  (bind _cube (`self.Cube`))
  (`KismetSystemLibrary.K2_SetTimerDelegate` (delegate `/Game/MyBlueprints/Interaction/Int_Interaction_Highlight.OnRayMiss`) 0.1)
  (`PrimitiveComponent.SetRenderCustomDepth` _cube true)
  (`PrimitiveComponent.SetCustomDepthStencilValue` _cube (`self.Value`)))

(event `/Game/MyBlueprints/Interaction/Int_Interaction_Highlight.OnRayMiss`
  (`PrimitiveComponent.SetRenderCustomDepth` (`self.Cube`) false))

(event `/Game/MyBlueprints/Interaction/Int_Interaction_switch.OnInteracted`
  (for _array_element (`self.Target`)
    (`SceneComponent.ToggleVisibility` (`Light.LightComponent` _array_element) false)))

(fn `UserConstructionScript`)